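; BP_Masterbox is a box Blueprint that stores an item and a count, and hands items out for placement.
; PlaceItemFromBox subtracts the requested amount from BoxedAmount when stock suffices, returning BoxedItem and that amount.
; An empty box returns zero.
; A request exceeding stock zeroes BoxedAmount before returning it, so it also reports zero rather than the remainder.
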(fn `PlaceItemFromBox`
  (params (AmountToPlace :type Integer))
  (returns (ItemToPlace :type "/Game/Assets/Blueprints/Items/DA_MasterItem Object Reference") (AmountItemsToPlace :type Integer))
  (bind _boxedamount (`self.BoxedAmount`))
  (bind _boxeditem (`self.BoxedItem`))
  (bind _returnvalue (- _boxedamount AmountToPlace))
  (if (== _boxedamount 0)
    (return (`self.BoxedItem`) 0)
    (elif (>= _returnvalue 0)
      (set `self.BoxedAmount` _returnvalue)
      (return _boxeditem AmountToPlace)
      (else
        (set `self.BoxedAmount` 0)
        (return _boxeditem _boxedamount)))))

(fn `UserConstructionScript`)