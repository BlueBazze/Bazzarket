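; Base shelf actor that displays a stocked item as a grid of instanced static meshes inside its ShelfArea bounds.
; SetItem applies the item's mesh and derives grid capacity from shelf size and scaled item size.
; PlaceItem converts the next instance index into a grid position until full.
; Construction rebuilds instances from StockedAmount; AddStock places instances directly, while RemoveStock only lowers the count.
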(fn `AddStock`
  (params (AmountToAdd :type Integer :default 1) (ItemToAdd :type "/Game/Assets/Blueprints/Items/DA_MasterItem Object Reference"))
  (bind _returnvalue (== (`InstancedStaticMeshComponent.GetInstanceCount` (`self.ISM_ShelfItems`)) 0))
  (bind _stockeditem (`self.StockedItem`)
    (:`then`
      (if (== ItemToAdd _stockeditem)
        (for _ (range 1 (+ AmountToAdd 1)) :!label _label
          (`self.PlaceItem` _stockeditem))
        (else
          (`KismetSystemLibrary.LogString` "Shelf contain another item"))))
    (:`else`
      (if (and (== (`self.StockedAmount`) 0) _returnvalue)
        (`self.SetItem` ItemToAdd :!label _label_2)
        (goto _label)
        (elif _returnvalue
          (set `self.StockedAmount` 0)
          (goto _label_2))))))

(fn `CalculateItemPositionFromIndex`
  (params (Index :type Integer))
  (returns (PositionInShelfGrid :type "Vector Structure"))
  (bind (_capacity_x _capacity_y) (`KismetMathLibrary.BreakVector` (`self.Capacity`)))
  (bind _returnvalue (* _capacity_x _capacity_y))
  (return (`KismetMathLibrary.Conv_IntVectorToVector` (make `IntVector` (+ (mod Index (`KismetMathLibrary.FTrunc` _capacity_x)) 1) (`KismetMathLibrary.FTrunc` (+ (/ (mod Index _returnvalue) _capacity_x) 1.0)) (+ (/ Index _returnvalue) 0)))))

(fn `CalculateShelfCapacity`
  (bind _stockeditem (`self.StockedItem`))
  (bind _size (`/Game/Assets/Blueprints/Items/DA_MasterItem.GetItemSize` _stockeditem))
  (bind _shelfvectorsize (`self.GetShelfSize`))
  (bind _x (.x _shelfvectorsize))
  (bind _y (.y _shelfvectorsize))
  (bind _z (.z _shelfvectorsize))
  (bind _returnvalue (/ _x (.x (* (/ _size 2) (`/Game/Assets/Blueprints/Items/DA_MasterItem.ItemScale` _stockeditem)))))
  (bind _returnvalue_2 (/ _y (.y (* (/ _size 2) (`/Game/Assets/Blueprints/Items/DA_MasterItem.ItemScale` _stockeditem)))))
  (bind _returnvalue_3 (/ _z (.z (* (/ _size 2) (`/Game/Assets/Blueprints/Items/DA_MasterItem.ItemScale` _stockeditem)))))
  (set `self.Capacity` (`KismetMathLibrary.MakeVector` (`KismetMathLibrary.Conv_IntToDouble` (`KismetMathLibrary.FFloor` _returnvalue)) (`KismetMathLibrary.Conv_IntToDouble` (`KismetMathLibrary.FFloor` _returnvalue_2)) (`KismetMathLibrary.Conv_IntToDouble` (`KismetMathLibrary.FFloor` _returnvalue_3))))
  (set `self.Spacing` (`KismetMathLibrary.MakeVector` (mod _x _returnvalue) (mod _y _returnvalue_2) (mod _z _returnvalue_3))))

(fn `GetShelfSize`
  (returns (ShelfVectorSize :type "Vector Structure"))
  (return (* (`.BoxExtent` (`KismetSystemLibrary.GetComponentBounds` (`self.ShelfArea`))) 2)))

(fn `PlaceItem`
  (params (ItemClass :type "/Game/Assets/Blueprints/Items/DA_MasterItem Object Reference"))
  (bind _itemsize (`self.ItemSize`))
  (bind (_capacity_x _capacity_y _capacity_z) (`KismetMathLibrary.BreakVector` (`self.Capacity`)))
  (bind _returnvalue (`InstancedStaticMeshComponent.GetInstanceCount` (`self.ISM_ShelfItems`)))
  (bind (_returnvalue_x _returnvalue_y) (`KismetMathLibrary.BreakVector` (/ _itemsize (1.0 2.0 1.0))))
  (bind _returnvalue_2 (* (* _capacity_x _capacity_y) _capacity_z))
  (if (< _returnvalue _returnvalue_2)
    (bind _positioninshelfgrid (`self.CalculateItemPositionFromIndex` _returnvalue))
    (`InstancedStaticMeshComponent.AddInstance` (`self.ISM_ShelfItems`) (`KismetMathLibrary.MakeTransform` (- (* (* _itemsize (`/Game/Assets/Blueprints/Items/DA_MasterItem.ItemScale` (`self.StockedItem`))) _positioninshelfgrid) (`KismetMathLibrary.MakeVector` _returnvalue_x _returnvalue_y)) (struct) (`KismetMathLibrary.Conv_DoubleToVector` (`/Game/Assets/Blueprints/Items/DA_MasterItem.ItemScale` (`self.StockedItem`)))) false)
    (else
      (set `self.StockedAmount` _returnvalue_2))))

(fn `RefreshStock`
  (if (!= (`InstancedStaticMeshComponent.GetInstanceCount` (`self.ISM_ShelfItems`)) (`self.StockedAmount`))
    (`InstancedStaticMeshComponent.ClearInstances` (`self.ISM_ShelfItems`))
    (if (> (`self.StockedAmount`) 0)
      (for _ (range (+ (`self.StockedAmount`) 1))
        (`self.PlaceItem` (`self.StockedItem`))))))

(fn `RemoveStock`
  (params (Amount :type Integer :default 1))
  (bind _output_get (set `self.StockedAmount` (- (`self.StockedAmount`) Amount))))

(fn `SetItem`
  (params (NewItemOnShelf :type "/Game/Assets/Blueprints/Items/DA_MasterItem Object Reference"))
  (bind _ism_shelfitems (`self.ISM_ShelfItems`))
  (`StaticMeshComponent.SetStaticMesh` _ism_shelfitems (`/Game/Assets/Blueprints/Items/DA_MasterItem.ItemMesh` NewItemOnShelf))
  (`PrimitiveComponent.SetBoundsScale` _ism_shelfitems 2.0)
  (bind _size (`/Game/Assets/Blueprints/Items/DA_MasterItem.GetItemSize` NewItemOnShelf))
  (set `self.ItemSize` _size)
  (`self.CalculateShelfCapacity`))

(fn `UserConstructionScript`
  (bind _stockeditem (`self.StockedItem`)
    (:`then`
      (`self.SetItem` _stockeditem)
      (`self.RefreshStock`))
    (:`else`)))